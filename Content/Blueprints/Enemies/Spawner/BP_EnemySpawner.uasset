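; Enemy spawner actor that periodically spawns enemies at points on a ring around its own location.
; On BeginPlay it spaces points evenly around the circle, keeping those that pass a downward trace and a navmesh projection.
; A looping timer, using rate and class from SpawnerParams entry 1, spawns one enemy at every kept point.
; The player's level-up event clears that timer, stopping spawning with no restart.
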(event `self.ReceiveBeginPlay`
  (bind (_value _returnvalue) (`BlueprintMapLibrary.Map_Find` (`self.SpawnerParams`) 1))
  (`self.CalculateSpawnersLocation` (`self.K2_GetActorLocation`))
  (bind _asbp_third_person_character (cast `/Game/ThirdPerson/Blueprints/BP_ThirdPersonCharacter` (`GameplayStatics.GetPlayerCharacter` 0)))
  (set `self.Player` _asbp_third_person_character)
  (if _returnvalue
    (bind _returnvalue_2 (`KismetSystemLibrary.K2_SetTimerDelegate` (delegate `SpawnEnemies`) (`.SpawnRate_5_8ECAD8644411FE487FFE649C699D3399` (break `/Game/Blueprints/Enemies/Spawner/Structs/FSpawnerParams` _value)) true))
    (set `self.SpawnTimer` _returnvalue_2)
    (add `/Game/ThirdPerson/Blueprints/BP_ThirdPersonCharacter.LevelUp` (`self.Player`) (delegate `HandleLeveling`))))

(event `HandleLeveling`
  (params (CurLevel :type Integer))
  (`self.StopSpawner`))

(event `SpawnEnemies`
  (for _array_element (`self.SpawnLocation`)
    (`|SpawnActorFromClass` (`.Enemy_6_8455C4EA4285B2A5B3982897FDAEB640` (break `/Game/Blueprints/Enemies/Spawner/Structs/FSpawnerParams` (`BlueprintMapLibrary.Map_Find` (`self.SpawnerParams`) 1))) (`KismetMathLibrary.MakeTransform` _array_element) "Undefined" "MultiplyWithRoot" null null)))

(event `self.ReceiveTick`
  (params (DeltaSeconds :type "Float (single-precision)")))

(fn `CalculateSpawnersLocation`
  (params (CenterPoint :type "Vector Structure"))
  (locals (Center :type "Vector Structure") (FoundLocation :type "Vector Structure"))
  (bind (_center_x _center_y _center_z) (`KismetMathLibrary.BreakVector` (`local.Center`)))
  (bind _spawnradius (`self.SpawnRadius`))
  (set `local.Center` CenterPoint)
  (for _index (range (`self.NumberOfSpawners`))
    (bind _returnvalue (/ (* (`KismetMathLibrary.Conv_IntToDouble` _index) (* 2 (`KismetMathLibrary.GetPI`))) (`self.NumberOfSpawners`)))
    (set `local.FoundLocation` (`KismetMathLibrary.MakeVector` (+ _center_x (* _spawnradius (`KismetMathLibrary.Cos` _returnvalue))) (+ _center_y (* _spawnradius (`KismetMathLibrary.Sin` _returnvalue))) _center_z))
    (if (`self.CheckNavmesh` (`local.FoundLocation`))
      (`KismetArrayLibrary.Array_Add` (`self.SpawnLocation`) (`local.FoundLocation`)))))

(fn `CheckNavmesh`
  (params (Point :type "Vector Structure"))
  (returns (IsOnNavmesh :type Boolean))
  (locals (CheckPointLocation :type "Vector Structure"))
  (bind (_checkpointlocation_x _checkpointlocation_y _checkpointlocation_z) (`KismetMathLibrary.BreakVector` (`local.CheckPointLocation`)))
  (bind _output_get (set `local.CheckPointLocation` Point))
  (bind (_outhit _returnvalue) (`KismetSystemLibrary.LineTraceSingle` :`Start` _output_get :`End` (`KismetMathLibrary.MakeVector` _checkpointlocation_x _checkpointlocation_y (- _checkpointlocation_z 1000.0)) :`TraceChannel` "TraceTypeQuery1" :`DrawDebugType` "Persistent"))
  (return (and _returnvalue (`.ReturnValue` (`NavigationSystemV1.K2_ProjectPointToNavigation` (`local.CheckPointLocation`) null null (0.0 0.0 1000.0))))))

(fn `StopSpawner`
  (`KismetSystemLibrary.K2_ClearAndInvalidateTimerHandle` (`self.SpawnTimer`)))

(fn `UserConstructionScript`)