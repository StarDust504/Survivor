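; BP_EnemyBase is a base enemy character that loads its stats from a data table and dies when its health runs out.
; On BeginPlay, InitialSetup reads the RowName row to set current health, damage and walk speed, printing a placeholder message if the row is missing.
; AnyDamage subtracts from health and destroys the actor at zero or below.
; Getter functions expose base damage and current health.
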(event `self.ReceiveBeginPlay`
  (`self.InitialSetup`))

(event `self.ReceiveAnyDamage`
  (params (Damage :type "Float (single-precision)") (DamageType :type "DamageType Object Reference") (InstigatedBy :type "Controller Object Reference") (DamageCauser :type "Actor Object Reference"))
  (set `self.CurHealth` (- (`self.CurHealth`) Damage))
  (if (<= (`self.CurHealth`) 0.0)
    (`self.K2_DestroyActor`)))

(event `self.ReceiveTick`
  (params (DeltaSeconds :type "Float (single-precision)")))

(fn `GetBaseDamage`
  (returns (Damage :type "Float (double-precision)"))
  (return (`self.Damage`)))

(fn `GetCurrentHealth`
  (returns (Health :type "Float (double-precision)"))
  (return (`self.CurHealth`)))

(fn `InitialSetup`
  (`/Engine/EditorBlueprintResources/StandardMacros.IsValid` (`self.Data`)
    (:`Is Valid`
      (bind _returnvalue (`|GetDataTableRow` (`self.Data`) (`self.RowName`))
        (:`then`
          (bind (_maxhealth _damage _speed) (break `/Game/Blueprints/Enemies/DataTables/Structures/FEnemyStats` _returnvalue))
          (set `self.CurHealth` _maxhealth)
          (set `self.Damage` _damage)
          (set `CharacterMovementComponent.MaxWalkSpeed` _speed (`self.CharacterMovement`)))
        (:`RowNotFound`
          (`KismetSystemLibrary.PrintString` "Hello"))))))

(fn `UserConstructionScript`)