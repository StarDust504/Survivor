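; Projectile actor that damages what it hits and credits kills to the instigator that fired it.
; Each tick it line traces on Visibility from its last position to its current one, with debug drawing, rather than relying on overlaps.
; The first hit stops movement, applies the instigator's base damage to I_Damage actors, increments the instigator's kill counter if health reaches zero, then destroys the projectile.
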(event `self.ReceiveBeginPlay`
  (set `self.PrevLocation` (`self.K2_GetActorLocation`)))

(event `self.ReceiveTick`
  (params (DeltaSeconds :type "Float (single-precision)"))
  (bind (_outhit _returnvalue) (`KismetSystemLibrary.LineTraceSingle` :`Start` (`self.PrevLocation`) :`End` (`self.K2_GetActorLocation`) :`TraceChannel` "TraceTypeQuery1" :`DrawDebugType` "ForDuration"))
  (if _returnvalue
    (`/Engine/EditorBlueprintResources/StandardMacros.DoOnce` false
      (:`Completed`
        (`ProjectileMovementComponent.StopSimulating` (`self.ProjectileMovement`) _outhit)
        (bind _damage (message `/Game/Interfaces/I_Damage.GetBaseDamage` (`self.GetInstigator`)))
        (bind (_bblockinghit _binitialoverlap _time _distance _location _impactpoint _normal _impactnormal _physmat _hitactor) (`GameplayStatics.BreakHitResult` _outhit))
        (if (`KismetSystemLibrary.DoesImplementInterface` _hitactor "/Game/Interfaces/I_Damage.I_Damage_C")
          (`GameplayStatics.ApplyDamage` _hitactor _damage null self)
          (bind _health (message `/Game/Interfaces/I_Damage.GetCurrentHealth` _hitactor))
          (if (<= _health 0.0)
            (message `/Game/Interfaces/I_Damage.IncreaseKillCounter` (`self.GetInstigator`))
            (`self.K2_DestroyActor`)
            (else
              (`self.K2_DestroyActor`)))
          (else
            (`self.K2_DestroyActor`)))))
    (else
      (set `self.PrevLocation` (`self.K2_GetActorLocation`)))))

(event `self.ReceiveActorBeginOverlap`
  (params (OtherActor :type "Actor Object Reference")))

(fn `UserConstructionScript`)