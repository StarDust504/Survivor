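; BP_Projectile is a projectile that damages actors implementing I_Damage and credits kills to its instigator.
; Each tick it line-traces from its previous location to its current one, so fast movement does not clip through walls.
; On the first hit, HandleCollision stops movement, applies the instigator's base damage, and destroys the projectile.
; If the target's health drops to zero, it sends the target's kill value to the instigator's kill counter.
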(event `self.ReceiveBeginPlay`
  (set `self.PrevLocation` (`self.K2_GetActorLocation`)))

(event `self.ReceiveTick`
  (params (DeltaSeconds :type "Float (single-precision)"))
  ; Traces projectile trajectory on tick to avoid projectiles clipping through walls on high speeds
  (bind (_outhit _returnvalue) (`KismetSystemLibrary.LineTraceSingle` (`self.PrevLocation`) (`self.K2_GetActorLocation`) "TraceTypeQuery1"))
  (if _returnvalue
    (`/Engine/EditorBlueprintResources/StandardMacros.DoOnce` false
      (:`Completed`
        (`self.HandleCollision` _outhit)))
    (else
      (set `self.PrevLocation` (`self.K2_GetActorLocation`)))))

(fn `HandleCollision`
  (params (HitResult :type "HitResult Structure"))
  (bind (_bblockinghit _binitialoverlap _time _distance _location _impactpoint _normal _impactnormal _physmat _hitactor) (`GameplayStatics.BreakHitResult` HitResult))
  ; When collision is detected applies damage to collided actor if it implements Damage interface, if damaged actor dies reports its death to a player to increase number of kiils and levelup
  (`ProjectileMovementComponent.StopSimulating` (`self.ProjectileMovement`) HitResult)
  (if (`KismetSystemLibrary.DoesImplementInterface` _hitactor "/Game/Interfaces/I_Damage.I_Damage_C")
    (bind _damage (message `/Game/Interfaces/I_Damage.GetBaseDamage` (`self.GetInstigator`)))
    (bind _value (message `/Game/Interfaces/I_Damage.GetKillValue` _hitactor))
    (`GameplayStatics.ApplyDamage` _hitactor _damage null self)
    (bind _health (message `/Game/Interfaces/I_Damage.GetCurrentHealth` _hitactor))
    (if (<= _health 0.0)
      (message `/Game/Interfaces/I_Damage.IncreaseKillCounter` (`self.GetInstigator`) _value)
      (`self.K2_DestroyActor`)
      (else
        (`self.K2_DestroyActor`)))
    (else
      (`self.K2_DestroyActor`))))

(fn `UserConstructionScript`)