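; BP_EnemyBase is the base enemy Blueprint, holding health, damage, movement speed and kill value for wave-based play.
; On BeginPlay it loads these stats from a named DataTable row.
; Incoming damage lowers health and destroys the actor at zero.
; It binds to the player's new-wave event, destroying itself when that fires with Started false, and exposes getters for damage, health and kill value.
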(event `self.ReceiveBeginPlay`
  ; Enemy setup
  (`self.InitialSetup`))

(event `self.ReceiveAnyDamage`
  (params (Damage :type "Float (single-precision)") (DamageType :type "DamageType Object Reference") (InstigatedBy :type "Controller Object Reference") (DamageCauser :type "Actor Object Reference"))
  ; Applies damage to enemy
  (set `self.CurHealth` (- (`self.CurHealth`) Damage))
  (if (<= (`self.CurHealth`) 0.0)
    (`self.K2_DestroyActor`)))

(event `PlayerRecieved`
  (params (Player :type "/Game/ThirdPerson/Blueprints/BP_ThirdPersonCharacter Object Reference"))
  ; Clear all enemies before a new wave
  (`/Engine/EditorBlueprintResources/StandardMacros.IsValid` Player
    (:`Is Valid`
      (add `/Game/ThirdPerson/Blueprints/BP_ThirdPersonCharacter.NewWave` Player (delegate `HandleNewWave`)))))

(event `HandleNewWave`
  (params (Started :type Boolean))
  ; Clear all enemies before a new wave
  (if (not Started)
    (`self.K2_DestroyActor`)))

(fn `GetBaseDamage`
  (returns (Damage :type "Float (double-precision)"))
  (return (`self.Damage`)))

(fn `GetCurrentHealth`
  (returns (Health :type "Float (double-precision)"))
  (return (`self.CurHealth`)))

(fn `GetKillValue`
  (returns (Value :type Integer))
  (return (`self.KillValue`)))

(fn `InitialSetup`
  ; Sets up all of the enemy stats from row in a DataTable
  (`/Engine/EditorBlueprintResources/StandardMacros.IsValid` (`self.Data`)
    (:`Is Valid`
      (bind _returnvalue (`|GetDataTableRow` (`self.Data`) (`self.RowName`))
        (:`then`
          (bind (_maxhealth _damage _speed _killcost) (break `/Game/Enemies/DataTables/Structures/FEnemyStats` _returnvalue))
          (set `self.CurHealth` _maxhealth)
          (set `self.Damage` _damage)
          (set `CharacterMovementComponent.MaxWalkSpeed` _speed (`self.CharacterMovement`))
          (set `self.KillValue` _killcost))))))

(fn `UserConstructionScript`)