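; Enemy spawner that periodically spawns a random enemy type at each point on a circle around itself, passing each enemy the player reference.
; On BeginPlay it computes evenly spaced points, keeping those that pass a downward trace and NavMesh projection, then starts a looping spawn timer.
; The player's new-wave event drives leveling: spawning stops for perk selection, then resumes at a faster rate.
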(event `self.ReceiveBeginPlay`
  ; Initial spawner setup: calculates spawn location, setups spawn timer
  (`self.CalculateSpawnersLocation` (`self.K2_GetActorLocation`))
  (bind _asbp_third_person_character (cast `/Game/ThirdPerson/Blueprints/BP_ThirdPersonCharacter` (`GameplayStatics.GetPlayerCharacter` 0)))
  (set `self.PlayerCharacter` _asbp_third_person_character)
  (`self.SetupEnemySpawner`)
  (add `/Game/ThirdPerson/Blueprints/BP_ThirdPersonCharacter.NewWave` (`self.PlayerCharacter`) (`|CreateDelegate` :!event `HandleLeveling`)))

(event `HandleLeveling`
  (params (Started :type Boolean))
  ; When player enters perk selection stage stops all of the spawners to clear out all of the enemies. When player confirms perk selection resets the timer with a faster spawn rate
  (if Started
    (bind _newrate (`/Game/ThirdPerson/Blueprints/BFL_SurvivorFunctionLib.IncreaseTimerRate` (`self.SpawnRate`) 1.1))
    (bind _output_get (set `self.SpawnRate` _newrate))
    (bind _returnvalue (`KismetSystemLibrary.K2_SetTimerDelegate` (`|CreateDelegate` :!event `SpawnEnemies`) _output_get true))
    (set `self.SpawnTimer` _returnvalue)
    (else
      (`self.StopSpawner`))))

(fn `CalculateSpawnersLocation`
  (params (CenterPoint :type "Vector Structure"))
  (locals (Center :type "Vector Structure") (FoundLocation :type "Vector Structure"))
  (bind (_center_x _center_y _center_z) (`KismetMathLibrary.BreakVector` (`local.Center`)))
  (bind _spawnradius (`self.SpawnRadius`))
  ; Calculates spawners location to make them evenly spread on a circle with a given radius and then checks if calculated spawner is on the ground and can reach Nav Mesh
  (set `local.Center` CenterPoint)
  (for _index (range (`self.NumberOfSpawners`))
    (bind _returnvalue (/ (* (`KismetMathLibrary.Conv_IntToDouble` _index) (* 2 (`KismetMathLibrary.GetPI`))) (`self.NumberOfSpawners`)))
    (set `local.FoundLocation` (`KismetMathLibrary.MakeVector` (+ _center_x (* _spawnradius (`KismetMathLibrary.Cos` _returnvalue))) (+ _center_y (* _spawnradius (`KismetMathLibrary.Sin` _returnvalue))) _center_z))
    (if (`self.CheckNavmesh` (`local.FoundLocation`))
      (`KismetArrayLibrary.Array_Add` (`self.SpawnLocation`) (`local.FoundLocation`)))))

(fn `CheckNavmesh`
  (params (Point :type "Vector Structure"))
  (returns (IsOnNavmesh :type Boolean))
  (locals (CheckPointLocation :type "Vector Structure"))
  (bind (_checkpointlocation_x _checkpointlocation_y _checkpointlocation_z) (`KismetMathLibrary.BreakVector` (`local.CheckPointLocation`)))
  ; Helper function to check if future spawn location can reach the ground and Nav Mesh
  (bind _output_get (set `local.CheckPointLocation` Point))
  (bind (_outhit _returnvalue) (`KismetSystemLibrary.LineTraceSingle` _output_get (`KismetMathLibrary.MakeVector` _checkpointlocation_x _checkpointlocation_y (- _checkpointlocation_z 1000.0)) "TraceTypeQuery1"))
  (return (and _returnvalue (`.ReturnValue` (`NavigationSystemV1.K2_ProjectPointToNavigation` (`local.CheckPointLocation`) null null (0.0 0.0 1000.0))))))

(fn `SetupEnemySpawner`
  ; Sets up enemy spawn timer and available enemy class array
  (set `self.EnemyClasses` (`|MakeArray` "/Game/Enemies/EnemyPresets/BP_EnemyOrdinary.BP_EnemyOrdinary_C" "/Game/Enemies/EnemyPresets/BP_EnemyDamage.BP_EnemyDamage_C" "/Game/Enemies/EnemyPresets/BP_EnemyFast.BP_EnemyFast_C" "/Game/Enemies/EnemyPresets/BP_EnemySlow.BP_EnemySlow_C" :!type "/Game/Enemies/BP_EnemyBase Class Reference"))
  (bind _returnvalue (`KismetSystemLibrary.K2_SetTimerDelegate` (`|CreateDelegate` :!event `SpawnEnemies`) (`self.SpawnRate`) true))
  (set `self.SpawnTimer` _returnvalue))

(fn `SpawnEnemies`
  ; For each valid spawn location picks a random enemy class and spawns it passing Player character ref to avoid Casts
  (for _array_element (`self.SpawnLocation`)
    (bind _returnvalue (`|SpawnActorFromClass` (`KismetArrayLibrary.Array_Random` (`self.EnemyClasses`)) (`KismetMathLibrary.MakeTransform` _array_element) "Undefined" "MultiplyWithRoot" null null))
    (`/Game/Enemies/BP_EnemyBase.PlayerRecieved` _returnvalue (`self.PlayerCharacter`))))

(fn `StopSpawner`
  ; We can call this function from outside of Spawner class to stop spawning enemies when Player died or entered perk selection stage
  (`KismetSystemLibrary.K2_ClearAndInvalidateTimerHandle` (`self.SpawnTimer`)))

(fn `UserConstructionScript`)